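; Character Blueprint for the red tennis player that leaves footstep decals on the ground while moving.
; Tick accumulates time while velocity is non-zero and resets it when the player stops.
; At each interval, a short downward object trace spawns a Decal_Footsteps actor at the impact point.
; Velocity is normalized before measuring, so the interval depends on StepsForVelocity rather than actual speed.
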(event EventBeginPlay)

(event Collision|EventActorBeginOverlap
  (params (OtherActor :type Actor%20Object%20Reference)))

(event EventTick
  (params (DeltaSeconds :type Float%20%28single-precision%29))
  (bind _returnvalue (Transformation|GetActorLocation))
  (bind _charactermovement (Variables|Character|GetCharacterMovement))
  (bind _velocity (Variables|/Script/Engine.MovementComponent|GetVelocity _charactermovement))
  (bind _returnvalue_2 (Math|Vector|Normalize _velocity))
  (bind _returnvalue_3 (Math|Vector|VectorLength _returnvalue_2))
  (Variables|Default|SetUpdateTime DeltaSeconds)
  (if (> _returnvalue_3 0.0)
    (bind _output_get (Variables|Default|SetUpdateTimeE (+ (Variables|Default|GetUpdateTimeE) (Variables|Default|GetUpdateTime))))
    (if (>= _output_get (/ _returnvalue_3 (Variables|Default|GetStepsForVelocity)))
      (bind (_outhit _returnvalue_4) (Collision|LineTraceForObjects _returnvalue (+ _returnvalue (* "0.000000,0.000000,-1.000000" 100)) (Utilities|Array|MakeArray "ObjectTypeQuery1" "ObjectTypeQuery2" "ObjectTypeQuery3" "ObjectTypeQuery4") false 0 "None"))
      (if _returnvalue_4
        (Game|SpawnActorfromClass "/Game/Blueprints/Decal_Footsteps.Decal_Footsteps_C" (Math|Conversions|ToTransform(Vector) (.ImpactPoint (Collision|BreakHitResult _outhit))) "Undefined" "MultiplyWithRoot" 0 0)
        (Variables|Default|SetUpdateTimeE 0.0)))
    (else
      (Variables|Default|SetUpdateTimeE 0.0))))

(fn ConstructionScript)